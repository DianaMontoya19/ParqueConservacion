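; BP_Quiz is a trigger box that freezes the first-person character and shows a quiz question when the character enters it.
; Begin overlap looks up RowName in the Questions DataTable, passes the row to the game mode's ShowQuizz, and switches to cursor-driven UI input.
; End overlap restores walking and calls HideQuizz, but sets UI-only input, visible cursor and ignored look again rather than restoring game controls.
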(event OnComponentBeginOverlap(Box)
  (params (OverlappedComponent :type Primitive%20Component%20Object%20Reference) (OtherActor :type Actor%20Object%20Reference) (OtherComp :type Primitive%20Component%20Object%20Reference) (OtherBodyIndex :type Integer) (bFromSweep :type Boolean) (SweepResult :type Hit%20Result%20Structure%20%28by%20ref%29))
  (bind _returnvalue (Game|GetPlayerController 0))
  (bind _asbp_first_person_character (Utilities|Casting|CastToBP_FirstPersonCharacter OtherActor))
  (Pawn|Components|CharacterMovement|SetMovementMode (Variables|/Script/Engine.Character|GetCharacterMovement _asbp_first_person_character) "MOVE_None" 0)
  (bind _returnvalue_2 (Utilities|GetDataTableRow (Variables|Default|GetQuestions) (Variables|Default|GetrowName))
    (:then
      (bind _asbp_first_person_game_mode (Utilities|Casting|CastToBP_FirstPersonGameMode (Game|GetGameMode)))
      (Default|ShowQuizz _asbp_first_person_game_mode _returnvalue_2)
      (Input|SetInputModeUIOnly _returnvalue 0 "DoNotLock" false)
      (Variables|/Script/Engine.PlayerController|SetbShowMouseCursor _returnvalue true)
      (Input|SetIgnoreLookInput _returnvalue true))
    (:RowNotFound
      (Development|PrintString "Row NO encontrada"))))

(event OnComponentEndOverlap(Box)
  (params (OverlappedComponent :type Primitive%20Component%20Object%20Reference) (OtherActor :type Actor%20Object%20Reference) (OtherComp :type Primitive%20Component%20Object%20Reference) (OtherBodyIndex :type Integer))
  (bind _returnvalue (Game|GetPlayerController 0))
  (bind _asbp_first_person_character (Utilities|Casting|CastToBP_FirstPersonCharacter OtherActor))
  (Pawn|Components|CharacterMovement|SetMovementMode (Variables|/Script/Engine.Character|GetCharacterMovement _asbp_first_person_character) "MOVE_Walking" 0)
  (Input|SetInputModeUIOnly _returnvalue (Variables|Default|GetWidget) "DoNotLock" false)
  (Variables|/Script/Engine.PlayerController|SetbShowMouseCursor _returnvalue true)
  (Input|SetIgnoreLookInput _returnvalue true)
  (bind _asbp_first_person_game_mode (Utilities|Casting|CastToBP_FirstPersonGameMode (Game|GetGameMode)))
  (Default|HideQuizz _asbp_first_person_game_mode))

(fn ConstructionScript)